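; BP_Doors is a two-panel door Blueprint that opens by moving its halves in opposite directions.
; OpenDoor applies equal and opposite local X offsets to two component groups, each holding a door panel, its decals and an edge-dirt component.
; The move is instant and unswept, with no animation, open-state check or close function, so repeated calls accumulate.
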(fn ConstructionScript)

(fn OpenDoor
  (Transformation|AddLocalOffset (Variables|Default|GetDecal1) "-70.000000,0.000000,0.000000" false false)
  (Transformation|AddLocalOffset (Variables|Default|GetDecal4) "70.000000,0.000000,0.000000" false false))