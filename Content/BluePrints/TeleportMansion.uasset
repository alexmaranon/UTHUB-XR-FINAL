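; Two-way teleporter actor for the mansion that moves the VR player between an upper and a lower point.
; Overlapping the CajaArriba or CajaAbajo trigger casts the other actor to BP_VRPawn, ignoring anything else.
; The pawn then snaps to the world location and rotation of the matching marker component, TpArriba or TpAbajo.
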(event OnComponentBeginOverlap(CajaArriba)
  (params (OverlappedComponent :type Primitive%20Component%20Object%20Reference) (OtherActor :type Actor%20Object%20Reference) (OtherComp :type Primitive%20Component%20Object%20Reference) (OtherBodyIndex :type Integer) (bFromSweep :type Boolean) (SweepResult :type Hit%20Result%20Structure%20%28by%20ref%29))
  (bind _tparriba (Variables|Default|GetTpArriba))
  (bind _asbp_vrpawn (Utilities|Casting|CastToBP_VRPawn OtherActor))
  (Transformation|SetActorLocationAndRotation _asbp_vrpawn (Transformation|GetWorldLocation _tparriba) (Transformation|GetWorldRotation _tparriba)))

(event OnComponentBeginOverlap(CajaAbajo)
  (params (OverlappedComponent :type Primitive%20Component%20Object%20Reference) (OtherActor :type Actor%20Object%20Reference) (OtherComp :type Primitive%20Component%20Object%20Reference) (OtherBodyIndex :type Integer) (bFromSweep :type Boolean) (SweepResult :type Hit%20Result%20Structure%20%28by%20ref%29))
  (bind _tpabajo (Variables|Default|GetTpAbajo))
  (bind _asbp_vrpawn (Utilities|Casting|CastToBP_VRPawn OtherActor))
  (Transformation|SetActorLocationAndRotation _asbp_vrpawn (Transformation|GetWorldLocation _tpabajo) (Transformation|GetWorldRotation _tpabajo)))

(event EventBeginPlay)

(event Collision|EventActorBeginOverlap
  (params (OtherActor :type Actor%20Object%20Reference)))

(event EventTick
  (params (DeltaSeconds :type Float%20%28single-precision%29)))

(fn ConstructionScript)