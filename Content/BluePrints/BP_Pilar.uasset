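; BP_Pilar is a puzzle checker that detects when every entry in its PuzzleOptions has the right key.
; BeginPlay starts a looping one-second timer, apparently to drive CheckPilar, which polls each option's RightKey flag.
; Once none is false, it prints a placeholder "GG" message and clears the timer to stop polling.
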(event Custom|CheckPilar
  (Variables|Default|SetIfFalse false)
  (for _array_element (Variables|Default|GetPuzzleOptions)
    (if (not (Variables|/Script/UTHUB_XR_1.PilarPuzzle|GetRightKey _array_element))
      (Variables|Default|SetIfFalse true)))
  (if (not (Variables|Default|GetIfFalse))
    (Development|PrintString "GG")
    (Utilities|Time|ClearandInvalidateTimerbyHandle (Variables|Default|GetTimerByEvent))))

(event EventBeginPlay
  (bind _returnvalue (Utilities|Time|SetTimerbyEvent (EventDispatchers|CreateEvent :!event Custom|CheckPilar) 1.0 true))
  (Variables|Default|SetTimerByEvent _returnvalue))

(fn ConstructionScript)