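; Keypad actor for the last minigame where a correct four-digit code calls MovePilars on a linked BP_Pilar.
; Per-pad overlaps, debounced by flags and a delayed release, nudge the pad and feed digits to AddValue; pad 9 enters 0.
; AddValue updates the displayed number and checks it at four digits, clearing on the next press.
; The light turns green and input locks on success, or red with an error sound on failure.
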(event OnComponentBeginOverlap(Coll_7)
  (params (OverlappedComponent :type Primitive%20Component%20Object%20Reference) (OtherActor :type Actor%20Object%20Reference) (OtherComp :type Primitive%20Component%20Object%20Reference) (OtherBodyIndex :type Integer) (bFromSweep :type Boolean) (SweepResult :type Hit%20Result%20Structure%20%28by%20ref%29))
  (if (not (Variables|Default|GetPressing7))
    (Variables|Default|SetPressing7 true)
    (CallFunction|AddValue (Class|KismetSystemLibrary|MakeLiteralInteger 7) (Variables|Default|GetPad7))))

(event OnComponentEndOverlap(Coll_7)
  (params (OverlappedComponent :type Primitive%20Component%20Object%20Reference) (OtherActor :type Actor%20Object%20Reference) (OtherComp :type Primitive%20Component%20Object%20Reference) (OtherBodyIndex :type Integer))
  (Utilities|FlowControl|Delay 0.1)
  (if (Variables|Default|GetPressing7)
    (Variables|Default|SetPressing7 false)
    (CallFunction|ExitButton (Variables|Default|GetPad7))))

(event OnComponentBeginOverlap(coll_4)
  (params (OverlappedComponent :type Primitive%20Component%20Object%20Reference) (OtherActor :type Actor%20Object%20Reference) (OtherComp :type Primitive%20Component%20Object%20Reference) (OtherBodyIndex :type Integer) (bFromSweep :type Boolean) (SweepResult :type Hit%20Result%20Structure%20%28by%20ref%29))
  (if (not (Variables|Default|GetPressing4))
    (Variables|Default|SetPressing4 true)
    (CallFunction|AddValue (Class|KismetSystemLibrary|MakeLiteralInteger 4) (Variables|Default|GetPad4))))

(event OnComponentEndOverlap(coll_4)
  (params (OverlappedComponent :type Primitive%20Component%20Object%20Reference) (OtherActor :type Actor%20Object%20Reference) (OtherComp :type Primitive%20Component%20Object%20Reference) (OtherBodyIndex :type Integer))
  (Utilities|FlowControl|Delay 0.1)
  (if (Variables|Default|GetPressing4)
    (Variables|Default|SetPressing4 false)
    (CallFunction|ExitButton (Variables|Default|GetPad4))))

(event OnComponentBeginOverlap(Coll_1)
  (params (OverlappedComponent :type Primitive%20Component%20Object%20Reference) (OtherActor :type Actor%20Object%20Reference) (OtherComp :type Primitive%20Component%20Object%20Reference) (OtherBodyIndex :type Integer) (bFromSweep :type Boolean) (SweepResult :type Hit%20Result%20Structure%20%28by%20ref%29))
  (if (not (Variables|Default|GetPressing1))
    (Variables|Default|SetPressing1 true)
    (CallFunction|AddValue (Class|KismetSystemLibrary|MakeLiteralInteger 1) (Variables|Default|GetPad1))))

(event OnComponentEndOverlap(Coll_1)
  (params (OverlappedComponent :type Primitive%20Component%20Object%20Reference) (OtherActor :type Actor%20Object%20Reference) (OtherComp :type Primitive%20Component%20Object%20Reference) (OtherBodyIndex :type Integer))
  (Utilities|FlowControl|Delay 0.1)
  (if (Variables|Default|GetPressing1)
    (Variables|Default|SetPressing1 false)
    (CallFunction|ExitButton (Variables|Default|GetPad1))))

(event OnComponentBeginOverlap(Coll_2)
  (params (OverlappedComponent :type Primitive%20Component%20Object%20Reference) (OtherActor :type Actor%20Object%20Reference) (OtherComp :type Primitive%20Component%20Object%20Reference) (OtherBodyIndex :type Integer) (bFromSweep :type Boolean) (SweepResult :type Hit%20Result%20Structure%20%28by%20ref%29))
  (if (not (Variables|Default|GetPressing2))
    (Variables|Default|SetPressing2 true)
    (CallFunction|AddValue (Class|KismetSystemLibrary|MakeLiteralInteger 2) (Variables|Default|GetPad2))))

(event OnComponentEndOverlap(Coll_2)
  (params (OverlappedComponent :type Primitive%20Component%20Object%20Reference) (OtherActor :type Actor%20Object%20Reference) (OtherComp :type Primitive%20Component%20Object%20Reference) (OtherBodyIndex :type Integer))
  (Utilities|FlowControl|Delay 0.1)
  (if (Variables|Default|GetPressing2)
    (Variables|Default|SetPressing2 false)
    (CallFunction|ExitButton (Variables|Default|GetPad2))))

(event OnComponentBeginOverlap(Coll_8)
  (params (OverlappedComponent :type Primitive%20Component%20Object%20Reference) (OtherActor :type Actor%20Object%20Reference) (OtherComp :type Primitive%20Component%20Object%20Reference) (OtherBodyIndex :type Integer) (bFromSweep :type Boolean) (SweepResult :type Hit%20Result%20Structure%20%28by%20ref%29))
  (if (not (Variables|Default|GetPressing8))
    (Variables|Default|SetPressing8 true)
    (CallFunction|AddValue (Class|KismetSystemLibrary|MakeLiteralInteger 8) (Variables|Default|GetPad8))))

(event OnComponentEndOverlap(Coll_8)
  (params (OverlappedComponent :type Primitive%20Component%20Object%20Reference) (OtherActor :type Actor%20Object%20Reference) (OtherComp :type Primitive%20Component%20Object%20Reference) (OtherBodyIndex :type Integer))
  (Utilities|FlowControl|Delay 0.1)
  (if (Variables|Default|GetPressing8)
    (Variables|Default|SetPressing8 false)
    (CallFunction|ExitButton (Variables|Default|GetPad8))))

(event OnComponentBeginOverlap(Coll_6)
  (params (OverlappedComponent :type Primitive%20Component%20Object%20Reference) (OtherActor :type Actor%20Object%20Reference) (OtherComp :type Primitive%20Component%20Object%20Reference) (OtherBodyIndex :type Integer) (bFromSweep :type Boolean) (SweepResult :type Hit%20Result%20Structure%20%28by%20ref%29))
  (if (not (Variables|Default|GetPressing6))
    (Variables|Default|SetPressing6 true)
    (CallFunction|AddValue (Class|KismetSystemLibrary|MakeLiteralInteger 6) (Variables|Default|GetPad6))))

(event OnComponentEndOverlap(Coll_6)
  (params (OverlappedComponent :type Primitive%20Component%20Object%20Reference) (OtherActor :type Actor%20Object%20Reference) (OtherComp :type Primitive%20Component%20Object%20Reference) (OtherBodyIndex :type Integer))
  (Utilities|FlowControl|Delay 0.1)
  (if (Variables|Default|GetPressing6)
    (Variables|Default|SetPressing6 false)
    (CallFunction|ExitButton (Variables|Default|GetPad6))))

(event OnComponentEndOverlap(coll_9)
  (params (OverlappedComponent :type Primitive%20Component%20Object%20Reference) (OtherActor :type Actor%20Object%20Reference) (OtherComp :type Primitive%20Component%20Object%20Reference) (OtherBodyIndex :type Integer))
  (Utilities|FlowControl|Delay 0.1)
  (if (Variables|Default|GetPressing9)
    (Variables|Default|SetPressing9 false)
    (CallFunction|ExitButton (Variables|Default|GetPad9))))

(event OnComponentBeginOverlap(coll_9)
  (params (OverlappedComponent :type Primitive%20Component%20Object%20Reference) (OtherActor :type Actor%20Object%20Reference) (OtherComp :type Primitive%20Component%20Object%20Reference) (OtherBodyIndex :type Integer) (bFromSweep :type Boolean) (SweepResult :type Hit%20Result%20Structure%20%28by%20ref%29))
  (if (not (Variables|Default|GetPressing9))
    (Variables|Default|SetPressing9 true)
    (CallFunction|AddValue (Class|KismetSystemLibrary|MakeLiteralInteger) (Variables|Default|GetPad9))))

(event OnComponentBeginOverlap(coll_5)
  (params (OverlappedComponent :type Primitive%20Component%20Object%20Reference) (OtherActor :type Actor%20Object%20Reference) (OtherComp :type Primitive%20Component%20Object%20Reference) (OtherBodyIndex :type Integer) (bFromSweep :type Boolean) (SweepResult :type Hit%20Result%20Structure%20%28by%20ref%29))
  (if (not (Variables|Default|GetPressing5))
    (Variables|Default|SetPressing5 true)
    (CallFunction|AddValue (Class|KismetSystemLibrary|MakeLiteralInteger 5) (Variables|Default|GetPad5))))

(event OnComponentEndOverlap(coll_5)
  (params (OverlappedComponent :type Primitive%20Component%20Object%20Reference) (OtherActor :type Actor%20Object%20Reference) (OtherComp :type Primitive%20Component%20Object%20Reference) (OtherBodyIndex :type Integer))
  (Utilities|FlowControl|Delay 0.1)
  (if (Variables|Default|GetPressing5)
    (Variables|Default|SetPressing5 false)
    (CallFunction|ExitButton (Variables|Default|GetPad5))))

(event OnComponentBeginOverlap(Coll_3)
  (params (OverlappedComponent :type Primitive%20Component%20Object%20Reference) (OtherActor :type Actor%20Object%20Reference) (OtherComp :type Primitive%20Component%20Object%20Reference) (OtherBodyIndex :type Integer) (bFromSweep :type Boolean) (SweepResult :type Hit%20Result%20Structure%20%28by%20ref%29))
  (if (not (Variables|Default|Getpressing3))
    (Variables|Default|Setpressing3 true)
    (CallFunction|AddValue (Class|KismetSystemLibrary|MakeLiteralInteger 3) (Variables|Default|GetPad3))))

(event OnComponentEndOverlap(Coll_3)
  (params (OverlappedComponent :type Primitive%20Component%20Object%20Reference) (OtherActor :type Actor%20Object%20Reference) (OtherComp :type Primitive%20Component%20Object%20Reference) (OtherBodyIndex :type Integer))
  (Utilities|FlowControl|Delay 0.1)
  (if (Variables|Default|Getpressing3)
    (Variables|Default|Setpressing3 false)
    (CallFunction|ExitButton (Variables|Default|GetPad3))))

(fn ConstructionScript)

(fn AddValue
  (params (NewItem :type Integer%20%28by%20ref%29) (Target :type Scene%20Component%20Object%20Reference))
  (bind _light (Variables|Default|GetLight))
  (Transformation|AddLocalOffset Target "-10.000000,0.000000,0.000000" false false)
  (if (not (Variables|Default|GetCorrectGuess))
    (Variables|Default|SetStringOfFloats "")
    (if (< (Utilities|Array|Length (Variables|Default|GetNumbersIntArray)) 4)
      _
      (else
        (Utilities|Array|Clear (Variables|Default|GetNumbersIntArray))))
    (Utilities|Array|Add (Variables|Default|GetNumbersIntArray) NewItem)
    (for _array_element (Variables|Default|GetNumbersIntArray)
      (Variables|Default|SetStringOfFloats (Utilities|String|Append (Variables|Default|GetStringOfFloats) (Utilities|String|ToString(Integer) _array_element))))
    (Rendering|Components|TextRender|SetText (Variables|Default|GetNumber) (Utilities|Text|ToText(String) (Variables|Default|GetStringOfFloats)))
    (if (== (Utilities|Array|Length (Variables|Default|GetNumbersIntArray)) 4)
      (bind _returnvalue (Class|Keypad|ActualValue (Variables|Default|GetStringOfFloats)))
      (if _returnvalue
        (Rendering|Material|SetMaterial _light 0 "/Game/Materials/M_Green.M_Green")
        (Variables|Default|SetCorrectGuess true)
        (bind _asbp_pilar (Utilities|Casting|CastToBP_Pilar (Variables|Default|GetSelectedDoor)))
        (Default|MovePilars _asbp_pilar)
        (else
          (Rendering|Material|SetMaterial _light 0 "/Game/Materials/M_Red.M_Red")
          (Audio|PlaySoundatLocation "/Game/AUDIO/Error.Error" (Transformation|GetActorLocation) "0, 0, 0" 1.0 1.0 0.0 0 0 0 0))))
    (return)))

(fn ExitButton
  (params (Target :type Scene%20Component%20Object%20Reference))
  (Transformation|AddLocalOffset Target "10.000000,0.000000,0.000000" false false))