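; BP_PilarPuzzle is a puzzle pillar that rises while a key-tagged actor overlaps it and drops when that actor leaves.
; After a short delay, MoveCol overlap events offset both PuzzleBox and MoveCol vertically without sweep, using CanMove as the raised-state flag.
; IsAttached, never set here, blocks raising and makes Tick disable collision on both components.
; Debug text prints on each move.
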(event OnComponentBeginOverlap(moveCol)
  (params (OverlappedComponent :type Primitive%20Component%20Object%20Reference) (OtherActor :type Actor%20Object%20Reference) (OtherComp :type Primitive%20Component%20Object%20Reference) (OtherBodyIndex :type Integer) (bFromSweep :type Boolean) (SweepResult :type Hit%20Result%20Structure%20%28by%20ref%29))
  (if (not (Variables|Default|GetCanMove))
    (if (not (Variables|Default|GetIsAttached))
      (if (Actor|ActorHasTag OtherActor "key")
        (Utilities|FlowControl|Delay 0.3)
        (Variables|Default|SetCanMove true)
        (Transformation|AddWorldOffset (Variables|Default|GetPuzzle_box) "0.000000,0.000000,80.000000" false false)
        (Development|PrintText "miau")))))

(event OnComponentEndOverlap(moveCol)
  (params (OverlappedComponent :type Primitive%20Component%20Object%20Reference) (OtherActor :type Actor%20Object%20Reference) (OtherComp :type Primitive%20Component%20Object%20Reference) (OtherBodyIndex :type Integer))
  (if (Variables|Default|GetCanMove)
    (if (Actor|ActorHasTag OtherActor "key")
      (Utilities|FlowControl|Delay 0.3)
      (Variables|Default|SetCanMove false)
      (Transformation|AddWorldOffset (Variables|Default|GetPuzzle_box) "0.000000,0.000000,-80.000000" false false)
      (Development|PrintText "Mew"))))

(event EventTick
  (params (DeltaSeconds :type Float%20%28single-precision%29))
  (if (Variables|Default|GetIsAttached)
    (Collision|SetCollisionEnabled (Variables|Default|GetPuzzle_box) "NoCollision")
    (else
      (Collision|SetCollisionEnabled (Variables|Default|GetmoveCol) "QueryAndPhysics"))))

(fn ConstructionScript)