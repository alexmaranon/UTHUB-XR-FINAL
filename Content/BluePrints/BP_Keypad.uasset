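; BP_Keypad is an in-world numeric keypad that opens a selected BP_Doors actor when the correct four-digit code is entered.
; End-overlap events on pads 1 to 9 pass their digit to AddValue, which shows the growing code as text and restarts after four digits.
; Each completed entry is checked by ActualValue, turning the light red or green; a correct guess opens the door and locks out further input.
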(event OnComponentEndOverlap(Pad8)
  (params (OverlappedComponent :type Primitive%20Component%20Object%20Reference) (OtherActor :type Actor%20Object%20Reference) (OtherComp :type Primitive%20Component%20Object%20Reference) (OtherBodyIndex :type Integer))
  (CallFunction|AddValue (Class|KismetSystemLibrary|MakeLiteralInteger 8)))

(event OnComponentEndOverlap(Pad4)
  (params (OverlappedComponent :type Primitive%20Component%20Object%20Reference) (OtherActor :type Actor%20Object%20Reference) (OtherComp :type Primitive%20Component%20Object%20Reference) (OtherBodyIndex :type Integer))
  (CallFunction|AddValue (Class|KismetSystemLibrary|MakeLiteralInteger 4)))

(event OnComponentEndOverlap(Pad1)
  (params (OverlappedComponent :type Primitive%20Component%20Object%20Reference) (OtherActor :type Actor%20Object%20Reference) (OtherComp :type Primitive%20Component%20Object%20Reference) (OtherBodyIndex :type Integer))
  (CallFunction|AddValue (Class|KismetSystemLibrary|MakeLiteralInteger 1)))

(event OnComponentEndOverlap(Pad3)
  (params (OverlappedComponent :type Primitive%20Component%20Object%20Reference) (OtherActor :type Actor%20Object%20Reference) (OtherComp :type Primitive%20Component%20Object%20Reference) (OtherBodyIndex :type Integer))
  (CallFunction|AddValue (Class|KismetSystemLibrary|MakeLiteralInteger 3)))

(event OnComponentEndOverlap(Pad2)
  (params (OverlappedComponent :type Primitive%20Component%20Object%20Reference) (OtherActor :type Actor%20Object%20Reference) (OtherComp :type Primitive%20Component%20Object%20Reference) (OtherBodyIndex :type Integer))
  (CallFunction|AddValue (Class|KismetSystemLibrary|MakeLiteralInteger 2)))

(event OnComponentEndOverlap(Pad9)
  (params (OverlappedComponent :type Primitive%20Component%20Object%20Reference) (OtherActor :type Actor%20Object%20Reference) (OtherComp :type Primitive%20Component%20Object%20Reference) (OtherBodyIndex :type Integer))
  (CallFunction|AddValue (Class|KismetSystemLibrary|MakeLiteralInteger 9)))

(event OnComponentEndOverlap(Pad6)
  (params (OverlappedComponent :type Primitive%20Component%20Object%20Reference) (OtherActor :type Actor%20Object%20Reference) (OtherComp :type Primitive%20Component%20Object%20Reference) (OtherBodyIndex :type Integer))
  (CallFunction|AddValue (Class|KismetSystemLibrary|MakeLiteralInteger 6)))

(event OnComponentEndOverlap(Pad5)
  (params (OverlappedComponent :type Primitive%20Component%20Object%20Reference) (OtherActor :type Actor%20Object%20Reference) (OtherComp :type Primitive%20Component%20Object%20Reference) (OtherBodyIndex :type Integer))
  (CallFunction|AddValue (Class|KismetSystemLibrary|MakeLiteralInteger 5)))

(event OnComponentEndOverlap(Pad7)
  (params (OverlappedComponent :type Primitive%20Component%20Object%20Reference) (OtherActor :type Actor%20Object%20Reference) (OtherComp :type Primitive%20Component%20Object%20Reference) (OtherBodyIndex :type Integer))
  (CallFunction|AddValue (Class|KismetSystemLibrary|MakeLiteralInteger 7)))

(fn ConstructionScript)

(fn AddValue
  (params (NewItem :type Integer%20%28by%20ref%29))
  (bind _light (Variables|Default|GetLight))
  (if (not (Variables|Default|GetCorrectGuess))
    (Variables|Default|SetStringOfFloats "")
    (if (< (Utilities|Array|Length (Variables|Default|GetNumbersIntArray)) 4)
      _
      (else
        (Utilities|Array|Clear (Variables|Default|GetNumbersIntArray))))
    (Utilities|Array|Add (Variables|Default|GetNumbersIntArray) NewItem)
    (for _array_element (Variables|Default|GetNumbersIntArray)
      (Variables|Default|SetStringOfFloats (Utilities|String|Append (Variables|Default|GetStringOfFloats) (Utilities|String|ToString(Integer) _array_element))))
    (Rendering|Components|TextRender|SetText (Variables|Default|GetNumber) (Utilities|Text|ToText(String) (Variables|Default|GetStringOfFloats)))
    (if (== (Utilities|Array|Length (Variables|Default|GetNumbersIntArray)) 4)
      (bind _returnvalue (Class|Keypad|ActualValue (Variables|Default|GetStringOfFloats)))
      (if _returnvalue
        (Rendering|Material|SetMaterial _light 0 "/Game/Materials/M_Green.M_Green")
        (Variables|Default|SetCorrectGuess true)
        (bind _asbp_doors (Utilities|Casting|CastToBP_Doors (Variables|Default|GetSelectedDoor)))
        (Default|OpenDoor _asbp_doors)
        (else
          (Rendering|Material|SetMaterial _light 0 "/Game/Materials/M_Red.M_Red"))))
    (return)))