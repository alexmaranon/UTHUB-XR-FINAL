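; Four-plate map puzzle button that reports progress to BP_PuzzleMapas.
; It randomly picks Spain or Peru, shuffles colour materials across four planes, and expects the green or pink plane's plate respectively.
; Overlaps animate plates via timelines, check materials and switch connected actors; solving one map shows the other.
; A looping timer calls Boton2 while both are solved; wrong-answer handling and the Mexico map's trigger are disconnected.
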(event OnComponentBeginOverlap(TriggerVolume)
  (params (OverlappedComponent :type Primitive%20Component%20Object%20Reference) (OtherActor :type Actor%20Object%20Reference) (OtherComp :type Primitive%20Component%20Object%20Reference) (OtherBodyIndex :type Integer) (bFromSweep :type Boolean) (SweepResult :type Hit%20Result%20Structure%20%28by%20ref%29))
  (CallFunction|OnPlate))

(event OnComponentEndOverlap(TriggerVolume)
  (params (OverlappedComponent :type Primitive%20Component%20Object%20Reference) (OtherActor :type Actor%20Object%20Reference) (OtherComp :type Primitive%20Component%20Object%20Reference) (OtherBodyIndex :type Integer))
  (Utilities|RunOffPlate
    (:True
      (CallFunction|OffPlate)
      (if true
        _))))

(event OnComponentBeginOverlap(TriggerVolume1)
  (params (OverlappedComponent :type Primitive%20Component%20Object%20Reference) (OtherActor :type Actor%20Object%20Reference) (OtherComp :type Primitive%20Component%20Object%20Reference) (OtherBodyIndex :type Integer) (bFromSweep :type Boolean) (SweepResult :type Hit%20Result%20Structure%20%28by%20ref%29))
  (CallFunction|OnPlate2))

(event OnComponentEndOverlap(TriggerVolume1)
  (params (OverlappedComponent :type Primitive%20Component%20Object%20Reference) (OtherActor :type Actor%20Object%20Reference) (OtherComp :type Primitive%20Component%20Object%20Reference) (OtherBodyIndex :type Integer))
  (Utilities|RunOffPlate
    (:True
      (CallFunction|OffPlate2))))

(event OnComponentBeginOverlap(TriggerVolume2)
  (params (OverlappedComponent :type Primitive%20Component%20Object%20Reference) (OtherActor :type Actor%20Object%20Reference) (OtherComp :type Primitive%20Component%20Object%20Reference) (OtherBodyIndex :type Integer) (bFromSweep :type Boolean) (SweepResult :type Hit%20Result%20Structure%20%28by%20ref%29))
  (CallFunction|OnPlate3))

(event OnComponentEndOverlap(TriggerVolume2)
  (params (OverlappedComponent :type Primitive%20Component%20Object%20Reference) (OtherActor :type Actor%20Object%20Reference) (OtherComp :type Primitive%20Component%20Object%20Reference) (OtherBodyIndex :type Integer))
  (Utilities|RunOffPlate
    (:True
      (CallFunction|OfPlate3))))

(event OnComponentBeginOverlap(TriggerVolume3)
  (params (OverlappedComponent :type Primitive%20Component%20Object%20Reference) (OtherActor :type Actor%20Object%20Reference) (OtherComp :type Primitive%20Component%20Object%20Reference) (OtherBodyIndex :type Integer) (bFromSweep :type Boolean) (SweepResult :type Hit%20Result%20Structure%20%28by%20ref%29))
  (CallFunction|OnPlate4))

(event OnComponentEndOverlap(TriggerVolume3)
  (params (OverlappedComponent :type Primitive%20Component%20Object%20Reference) (OtherActor :type Actor%20Object%20Reference) (OtherComp :type Primitive%20Component%20Object%20Reference) (OtherBodyIndex :type Integer))
  (Utilities|RunOffPlate
    (:True
      (CallFunction|OffPlate4))))

(event Custom|SelecionMapa
  (bind _mapasaleatorios (Variables|Default|GetMapasAleatorios))
  (Utilities|Array|Shuffle _mapasaleatorios)
  (bind _output_get (Variables|Default|SetGuardarValorMapa (Utilities|Array|Get(acopy) _mapasaleatorios 1)))
  (Utilities|FlowControl|Sequence
    (:then_0
      (if (== (Variables|Default|GetGuardarValorMapa) 0)
        (CallFunction|ActivarPrimerMapa)
        (Variables|Default|SetContadorDeMapas (+ (Variables|Default|GetContadorDeMapas) 1) :!label _label)))
    (:then_1
      (if (== (Variables|Default|GetGuardarValorMapa) 1)
        (CallFunction|ActivarSegundoMapa)
        (goto _label)))))

(event Custom|ActivarSegundoMapa
  (bind _valoresaleatorios (Variables|Default|GetValoresAleatorios))
  (Variables|Default|SetEstoyMapa2 true)
  (Rendering|Material|SetMaterial (Variables|Default|GetMapaGeneral) 0 "/Game/Diego/Colores/peru.peru")
  (Utilities|Array|Shuffle _valoresaleatorios)
  (bind _output_get (Variables|Default|SetCogerValoresAleatorios _valoresaleatorios))
  (for (_array_element _array_index) _output_get
    (bind _output_get_2 (Variables|Default|SetRecogerColores (Utilities|Array|Get(acopy) (Variables|Default|GetColoresMapa2) _array_element)))
    (Rendering|Material|SetMaterial (Utilities|Array|Get(acopy) (Utilities|Array|MakeArray (Variables|Default|GetPlane) (Variables|Default|GetPlane1) (Variables|Default|GetPlane2) (Variables|Default|GetPlane3)) _array_index) 0 (Utilities|Array|Get(acopy) (Variables|Default|GetColoresMapa2) _array_element))))

(event Custom|On%20Plate2
  (bind _plane1 (Variables|Default|GetPlane1))
  (Variables|Runtime|SetState (not (Variables|Init|GetInvert)))
  (bind _alpha (Timeline|Timeline Play)
    (:Update
      (Transformation|SetRelativeLocation (Variables|Default|GetSM_Button_Top1) (Math|Vector|Lerp(Vector) "110.000000,0.000000,0.000000" "110.000000,0.000000,-5.000000" _alpha) false false))
    (:Button%20Press
      (if (not (Variables|Runtime|GetState))
        (CallFunction|SetStateOff)
        (Utilities|FlowControl|Sequence
          (:then_0
            (if (not (Variables|Default|GetSeCompletoMapa1))
              (if (and (== (Rendering|Material|GetMaterial _plane1 0) "/Game/Diego/Imagenes/1/MatVerde.MatVerde") (Variables|Default|GetEstoyMapa1))
                (CallFunction|PrimerMapaCompletado)
                (Variables|Default|SetLedi1 true)
                (CallFunction|SyncState :!label _label))))
          (:then_1
            (if (not (Variables|Default|GetSeCompletoMapa2))
              (if (and (== (Rendering|Material|GetMaterial _plane1 0) "/Game/Diego/Imagenes/2/MatRosa.MatRosa") (Variables|Default|GetEstoyMapa2))
                (CallFunction|SegundoMapaCompletado)
                (Variables|Default|SetLedi2 true)
                (goto _label)))))
        (else
          (CallFunction|SetStateon)
          (goto _label))))))

(event Custom|off%20plate%202
  (bind _plane1 (Variables|Default|GetPlane1))
  (Variables|Runtime|SetState (Variables|Init|GetInvert))
  (bind _alpha (Timeline|Timeline Reverse)
    (:Update
      (Transformation|SetRelativeLocation (Variables|Default|GetSM_Button_Top1) (Math|Vector|Lerp(Vector) "110.000000,0.000000,0.000000" "110.000000,0.000000,-5.000000" _alpha) false false))
    (:Button%20Press
      (if (not (Variables|Runtime|GetState))
        (CallFunction|SetStateOff)
        (Utilities|FlowControl|Sequence
          (:then_0
            (if (not (Variables|Default|GetSeCompletoMapa1))
              (if (and (== (Rendering|Material|GetMaterial _plane1 0) "/Game/Diego/Imagenes/1/MatVerde.MatVerde") (Variables|Default|GetEstoyMapa1))
                (CallFunction|PrimerMapaCompletado)
                (Variables|Default|SetLedi1 true)
                (CallFunction|SyncState :!label _label))))
          (:then_1
            (if (not (Variables|Default|GetSeCompletoMapa2))
              (if (and (== (Rendering|Material|GetMaterial _plane1 0) "/Game/Diego/Imagenes/2/MatRosa.MatRosa") (Variables|Default|GetEstoyMapa2))
                (CallFunction|SegundoMapaCompletado)
                (Variables|Default|SetLedi2 true)
                (goto _label)))))
        (else
          (CallFunction|SetStateon)
          (goto _label))))))

(event Custom|MapaFallado
  (Variables|Default|SetContadorDeMapas 0)
  (CallFunction|SelecionMapa)
  (Variables|Default|SetEstoyMapa1 false)
  (Variables|Default|SetEstoyMapa2 false))

(event Custom|On%20Plate3
  (bind _plane2 (Variables|Default|GetPlane2))
  (Variables|Runtime|SetState (not (Variables|Init|GetInvert)))
  (bind _alpha (Timeline|Timeline_0 Play)
    (:Update
      (Transformation|SetRelativeLocation (Variables|Default|GetSM_Button_Top2) (Math|Vector|Lerp(Vector) "0.000000,80.000000,0.000000" "0.000000,80.000000,-5.000000" _alpha) false false))
    (:Button%20Press
      (if (not (Variables|Runtime|GetState))
        (CallFunction|SetStateOff)
        (Utilities|FlowControl|Sequence
          (:then_0
            (if (not (Variables|Default|GetSeCompletoMapa1))
              (if (and (== (Rendering|Material|GetMaterial _plane2 0) "/Game/Diego/Imagenes/1/MatVerde.MatVerde") (Variables|Default|GetEstoyMapa1))
                (CallFunction|PrimerMapaCompletado)
                (Variables|Default|SetLedi1 true)
                (CallFunction|SyncState :!label _label))))
          (:then_1
            (if (not (Variables|Default|GetSeCompletoMapa2))
              (if (and (== (Rendering|Material|GetMaterial _plane2 0) "/Game/Diego/Imagenes/2/MatRosa.MatRosa") (Variables|Default|GetEstoyMapa2))
                (CallFunction|SegundoMapaCompletado)
                (Variables|Default|SetLedi2 true)
                (goto _label)))))
        (else
          (CallFunction|SetStateon)
          (goto _label))))))

(event Custom|of%20plate%203
  (bind _plane2 (Variables|Default|GetPlane2))
  (Variables|Runtime|SetState (Variables|Init|GetInvert))
  (bind _alpha (Timeline|Timeline_0 Reverse)
    (:Update
      (Transformation|SetRelativeLocation (Variables|Default|GetSM_Button_Top2) (Math|Vector|Lerp(Vector) "0.000000,80.000000,0.000000" "0.000000,80.000000,-5.000000" _alpha) false false))
    (:Button%20Press
      (if (not (Variables|Runtime|GetState))
        (CallFunction|SetStateOff)
        (Utilities|FlowControl|Sequence
          (:then_0
            (if (not (Variables|Default|GetSeCompletoMapa1))
              (if (and (== (Rendering|Material|GetMaterial _plane2 0) "/Game/Diego/Imagenes/1/MatVerde.MatVerde") (Variables|Default|GetEstoyMapa1))
                (CallFunction|PrimerMapaCompletado)
                (Variables|Default|SetLedi1 true)
                (CallFunction|SyncState :!label _label))))
          (:then_1
            (if (not (Variables|Default|GetSeCompletoMapa2))
              (if (and (== (Rendering|Material|GetMaterial _plane2 0) "/Game/Diego/Imagenes/2/MatRosa.MatRosa") (Variables|Default|GetEstoyMapa2))
                (CallFunction|SegundoMapaCompletado)
                (Variables|Default|SetLedi2 true)
                (goto _label)))))
        (else
          (CallFunction|SetStateon)
          (goto _label))))))

(event Custom|on%20plate%204
  (bind _plane3 (Variables|Default|GetPlane3))
  (Variables|Runtime|SetState (not (Variables|Init|GetInvert)))
  (bind _alpha (Timeline|Timeline_1 Play)
    (:Update
      (Transformation|SetRelativeLocation (Variables|Default|GetSM_Button_Top3) (Math|Vector|Lerp(Vector) "110.000000,80.000000,0.000000" "110.000000,80.000000,-5.000000" _alpha) false false))
    (:Button%20Press
      (if (not (Variables|Runtime|GetState))
        (CallFunction|SetStateOff)
        (Utilities|FlowControl|Sequence
          (:then_0
            (if (not (Variables|Default|GetSeCompletoMapa1))
              (if (and (== (Rendering|Material|GetMaterial _plane3 0) "/Game/Diego/Imagenes/1/MatVerde.MatVerde") (Variables|Default|GetEstoyMapa1))
                (CallFunction|PrimerMapaCompletado)
                (Variables|Default|SetLedi1 true)
                (CallFunction|SyncState :!label _label))))
          (:then_1
            (if (not (Variables|Default|GetSeCompletoMapa2))
              (if (and (== (Rendering|Material|GetMaterial _plane3 0) "/Game/Diego/Imagenes/2/MatRosa.MatRosa") (Variables|Default|GetEstoyMapa2))
                (CallFunction|SegundoMapaCompletado)
                (Variables|Default|SetLedi2 true)
                (goto _label)))))
        (else
          (CallFunction|SetStateon)
          (goto _label))))))

(event Custom|BloquearCollisionMapas
  (Collision|SetCollisionProfileName (Variables|Default|GetPlane) "NoCollision" true :!class /Script/Engine.PrimitiveComponent))

(event Custom|DesbloquearCollisionMapas
  (Collision|SetCollisionProfileName (Variables|Default|GetPlane1) "OverlapAll" true :!class /Script/Engine.PrimitiveComponent))

(event Custom|CustomEvent
  (if (and (Variables|Default|GetLedi1) (Variables|Default|GetLedi2))
    (Development|PrintString "Hello")
    (Default|Boton2 (CallFunction|GetRefMapas))))

(event Custom|off%20plate%204
  (bind _plane3 (Variables|Default|GetPlane3))
  (Variables|Runtime|SetState (Variables|Init|GetInvert))
  (bind _alpha (Timeline|Timeline_1 Reverse)
    (:Update
      (Transformation|SetRelativeLocation (Variables|Default|GetSM_Button_Top3) (Math|Vector|Lerp(Vector) "110.000000,80.000000,0.000000" "110.000000,80.000000,-5.000000" _alpha) false false))
    (:Button%20Press
      (if (not (Variables|Runtime|GetState))
        (CallFunction|SetStateOff)
        (Utilities|FlowControl|Sequence
          (:then_0
            (if (not (Variables|Default|GetSeCompletoMapa1))
              (if (and (== (Rendering|Material|GetMaterial _plane3 0) "/Game/Diego/Imagenes/1/MatVerde.MatVerde") (Variables|Default|GetEstoyMapa1))
                (CallFunction|PrimerMapaCompletado)
                (Variables|Default|SetLedi1 true)
                (CallFunction|SyncState :!label _label))))
          (:then_1
            (if (not (Variables|Default|GetSeCompletoMapa2))
              (if (and (== (Rendering|Material|GetMaterial _plane3 0) "/Game/Diego/Imagenes/2/MatRosa.MatRosa") (Variables|Default|GetEstoyMapa2))
                (CallFunction|SegundoMapaCompletado)
                (Variables|Default|SetLedi2 true)
                (goto _label)))))
        (else
          (CallFunction|SetStateon)
          (goto _label))))))

(event Custom|PrimerMapaCompletado
  (Default|Boton1 (CallFunction|GetRefMapas))
  (CallFunction|ActivarSegundoMapa)
  (Variables|Default|SetContadorDeMapas (+ (Variables|Default|GetContadorDeMapas) 1))
  (Variables|Default|SetSeCompletoMapa1 true)
  (Variables|Default|SetEstoyMapa1 false))

(event Custom|ActivarTercerMapa
  (bind _valoresaleatorios (Variables|Default|GetValoresAleatorios))
  (Variables|Default|SetEstoyMapa3 true)
  (Rendering|Material|SetMaterial (Variables|Default|GetMapaGeneral) 0 "/Game/Diego/Colores/mexico.mexico")
  (Utilities|Array|Shuffle _valoresaleatorios)
  (bind _output_get (Variables|Default|SetCogerValoresAleatorios _valoresaleatorios))
  (for (_array_element _array_index) _output_get
    (Variables|Default|SetRecogerColores (Utilities|Array|Get(acopy) (Variables|Default|GetColoresMapa3) _array_element))
    (Rendering|Material|SetMaterial (Utilities|Array|Get(acopy) (Utilities|Array|MakeArray (Variables|Default|GetPlane) (Variables|Default|GetPlane1) (Variables|Default|GetPlane2) (Variables|Default|GetPlane3)) _array_index) 0 (Utilities|Array|Get(acopy) (Variables|Default|GetColoresMapa3) _array_element))))

(event Custom|On%20Plate
  (Variables|Runtime|SetState (not (Variables|Init|GetInvert)))
  (bind _alpha (Timeline|Timeline_ButtonAnimation Play)
    (:Update
      (Transformation|SetRelativeLocation (Variables|Default|GetSM_Button_Top) (Math|Vector|Lerp(Vector) "0, 0, 0" "0, 0,-5.000000" _alpha) false false))
    (:Button%20Press
      (if (not (Variables|Runtime|GetState))
        (CallFunction|SetStateOff)
        (Utilities|FlowControl|Sequence
          (:then_0
            (if (not (Variables|Default|GetSeCompletoMapa1))
              (if (and (== (Rendering|Material|GetMaterial (Variables|Default|GetPlane) 0) "/Game/Diego/Imagenes/1/MatVerde.MatVerde") (Variables|Default|GetEstoyMapa1))
                (CallFunction|PrimerMapaCompletado)
                (Variables|Default|SetLedi1 true)
                (Variables|Default|SetEstoyMapa1 false)
                (CallFunction|SyncState :!label _label))))
          (:then_1
            (if (not (Variables|Default|GetSeCompletoMapa2))
              (if (and (== (Rendering|Material|GetMaterial (Variables|Default|GetPlane) 0) "/Game/Diego/Imagenes/2/MatRosa.MatRosa") (Variables|Default|GetEstoyMapa2))
                (CallFunction|SegundoMapaCompletado)
                (Variables|Default|SetLedi2 true)
                (Variables|Default|SetEstoyMapa2 false)
                (goto _label)))))
        (else
          (CallFunction|SetStateon)
          (goto _label))))))

(event Custom|Off%20Plate
  (Variables|Runtime|SetState (Variables|Init|GetInvert))
  (bind _alpha (Timeline|Timeline_ButtonAnimation Reverse)
    (:Update
      (Transformation|SetRelativeLocation (Variables|Default|GetSM_Button_Top) (Math|Vector|Lerp(Vector) "0, 0, 0" "0, 0,-5.000000" _alpha) false false))
    (:Button%20Press
      (if (not (Variables|Runtime|GetState))
        (CallFunction|SetStateOff)
        (Utilities|FlowControl|Sequence
          (:then_0
            (if (not (Variables|Default|GetSeCompletoMapa1))
              (if (and (== (Rendering|Material|GetMaterial (Variables|Default|GetPlane) 0) "/Game/Diego/Imagenes/1/MatVerde.MatVerde") (Variables|Default|GetEstoyMapa1))
                (CallFunction|PrimerMapaCompletado)
                (Variables|Default|SetLedi1 true)
                (Variables|Default|SetEstoyMapa1 false)
                (CallFunction|SyncState :!label _label))))
          (:then_1
            (if (not (Variables|Default|GetSeCompletoMapa2))
              (if (and (== (Rendering|Material|GetMaterial (Variables|Default|GetPlane) 0) "/Game/Diego/Imagenes/2/MatRosa.MatRosa") (Variables|Default|GetEstoyMapa2))
                (CallFunction|SegundoMapaCompletado)
                (Variables|Default|SetLedi2 true)
                (Variables|Default|SetEstoyMapa2 false)
                (goto _label)))))
        (else
          (CallFunction|SetStateon)
          (goto _label))))))

(event Custom|ActivarPrimerMapa
  (bind _valoresaleatorios (Variables|Default|GetValoresAleatorios))
  (Variables|Default|SetEstoyMapa1 true)
  (Rendering|Material|SetMaterial (Variables|Default|GetMapaGeneral) 0 "/Game/Diego/Colores/Espana.Espana")
  (Utilities|Array|Shuffle _valoresaleatorios)
  (bind _output_get (Variables|Default|SetCogerValoresAleatorios _valoresaleatorios))
  (Variables|Default|SetRecogerResultadoMapa1 (Utilities|Array|Get(acopy) _valoresaleatorios))
  (for (_array_element _array_index) _output_get
    (Variables|Default|SetRecogerColores (Utilities|Array|Get(acopy) (Variables|Default|GetColoresMapa1) _array_element))
    (Rendering|Material|SetMaterial (Utilities|Array|Get(acopy) (Utilities|Array|MakeArray (Variables|Default|GetPlane) (Variables|Default|GetPlane1) (Variables|Default|GetPlane2) (Variables|Default|GetPlane3)) _array_index) 0 (Utilities|Array|Get(acopy) (Variables|Default|GetColoresMapa1) _array_element))))

(event Custom|SegundoMapaCompletado
  (Default|Boton1 (CallFunction|GetRefMapas))
  (CallFunction|ActivarPrimerMapa)
  (Variables|Default|SetContadorDeMapas (+ (Variables|Default|GetContadorDeMapas) 1))
  (Variables|Default|SetSeCompletoMapa2 true)
  (Variables|Default|SetEstoyMapa2 false))

(event EventBeginPlay
  (CallFunction|SelecionMapa)
  (Utilities|Time|SetTimerbyEvent (delegate Custom|CustomEvent) 0.1 true))

(event EventTick
  (params (DeltaSeconds :type Float%20%28single-precision%29))
  (Development|PrintString (Utilities|String|ToString(Boolean) (== (Rendering|Material|GetMaterial (Variables|Default|GetPlane) 0) "/Game/Diego/Imagenes/1/MatVerde.MatVerde"))))

(event EventSyncInputState
  (params (State :type Boolean))
  (Variables|Runtime|SetState State))

(fn ConstructionScript)

(fn SetStateOff
  (for _array_element (Variables|Data|GetConnections)
    (Default|Off _array_element)))

(fn SetStateon
  (for _array_element (Variables|Data|GetConnections)
    (Default|On _array_element)))

(fn SyncState
  (for _array_element (Variables|Data|GetInput%20Sync)
    (Class|BPIInteraction|SyncInputState(Message) _array_element (Variables|Runtime|GetState))))

(fn GetRefMapas
  (Variables|Default|GetAs%20BP%20Puzzle%20Mapas
    (:then
      _)
    (:else
      (bind _asbp_puzzle_mapas (Utilities|Casting|CastToBP_PuzzleMapas (Variables|Default|GetRef)))
      (Variables|Default|SetAs%20BP%20Puzzle%20Mapas _asbp_puzzle_mapas)))
  (return (Variables|Default|GetAs%20BP%20Puzzle%20Mapas)))

(fn GetFractureBool
  (return false))

(fn GetItemType
  (return "NewEnumerator0"))

(fn GetMesh
  (return 0))