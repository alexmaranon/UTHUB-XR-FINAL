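; BP_PuzzleMapas is a three-step map puzzle that shows progress with three indicator lights, all red at BeginPlay.
; Each Boton event turns its light green; the first also swaps Mapa1 for Mapa2, and the second calls ActivarLuzPuerta on a referenced BP_Window_02.
; The first two events also set active flags.
; FallarPuzle turns all lights red without resetting the flags or maps.
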(event Custom|Boton1
  (Rendering|Material|SetMaterial (Variables|Default|GetLuz1) 0 "/Game/Diego/Colores/Verde.Verde")
  (Variables|Default|SetLuz1Activa true)
  (Rendering|SetVisibility (Variables|Default|GetMapa1) false false)
  (Rendering|SetVisibility (Variables|Default|GetMapa2) true false))

(event Custom|Boton2
  (Rendering|Material|SetMaterial (Variables|Default|Getluz2) 0 "/Game/Diego/Colores/Verde.Verde")
  (Variables|Default|SetLuz2Activa true)
  (bind _asbp_window_02 (Utilities|Casting|CastToBP_Window_02 (Variables|Default|GetActorRef)))
  (Default|ActivarLuzPuerta _asbp_window_02))

(event Custom|Boton3
  (Rendering|Material|SetMaterial (Variables|Default|GetLuz3) 0 "/Game/Diego/Colores/Verde.Verde"))

(event Custom|FallarPuzle
  (Rendering|Material|SetMaterial (Variables|Default|GetLuz1) 0 "/Game/Diego/Colores/Rojo.Rojo"))

(event EventBeginPlay
  (Rendering|Material|SetMaterial (Variables|Default|GetLuz3) 0 "/Game/Diego/Colores/Rojo.Rojo"))

(fn ConstructionScript)