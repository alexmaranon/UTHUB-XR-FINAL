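; Trigger-volume actor that moves the VR pawn to a child actor's location and rotation while its box is overlapped and the pawn's EstoyDentro flag is false.
; Box begin and end overlap events toggle Dentro without filtering which actor overlaps.
; A fast looping timer started on BeginPlay polls Dentro, checks the flag on player 0's BP_VRPawn and repeats the relocation while both conditions hold.
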(event OnComponentBeginOverlap(Box)
  (params (OverlappedComponent :type Primitive%20Component%20Object%20Reference) (OtherActor :type Actor%20Object%20Reference) (OtherComp :type Primitive%20Component%20Object%20Reference) (OtherBodyIndex :type Integer) (bFromSweep :type Boolean) (SweepResult :type Hit%20Result%20Structure%20%28by%20ref%29))
  (Variables|Default|SetDentro true))

(event OnComponentEndOverlap(Box)
  (params (OverlappedComponent :type Primitive%20Component%20Object%20Reference) (OtherActor :type Actor%20Object%20Reference) (OtherComp :type Primitive%20Component%20Object%20Reference) (OtherBodyIndex :type Integer))
  (Variables|Default|SetDentro false))

(event Custom|CustomEvent
  (bind _childactor (Variables|Default|GetChildActor))
  (if (Variables|Default|GetDentro)
    (bind _asbp_vrpawn (Utilities|Casting|CastToBP_VRPawn (Game|Player|GetPlayerPawn 0)))
    (if (not (Variables|/Game/BluePrints/BP_VRPawn.BP_VRPawn_C|GetEstoyDentro _asbp_vrpawn))
      (Transformation|SetActorLocationAndRotation _asbp_vrpawn (Transformation|GetWorldLocation _childactor) (Transformation|GetWorldRotation _childactor)))))

(event EventBeginPlay
  (Utilities|Time|SetTimerbyEvent (delegate Custom|CustomEvent) 0.1 true))

(fn ConstructionScript)