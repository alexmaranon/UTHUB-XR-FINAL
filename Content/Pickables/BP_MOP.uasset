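; BP_MOP is a mop from the Pickables folder that fades blood stains in front of it.
; BeginPlay starts a looping two-second timer, and the Patata event runs a short, offset line trace along the Cube's forward vector on the Visibility channel.
; A hit actor tagged Blood is cast to BP_BloodM and has LowerOpacity called on it.
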(event Custom|Patata
  (bind _returnvalue (Transformation|GetActorLocation))
  (bind _cube (Variables|Default|GetCube))
  (bind (_outhit _returnvalue_2) (Collision|LineTraceByChannel (+ _returnvalue (* (Math|Vector|GetForwardVector _cube) 7e+01)) (+ _returnvalue (* (Math|Vector|GetForwardVector _cube) 1.3e+02)) "TraceTypeQuery1" true 0 "None"))
  (if _returnvalue_2
    (if (Actor|ActorHasTag (.HitActor (Collision|BreakHitResult _outhit)) "Blood")
      (bind _asbp_blood_m (Utilities|Casting|CastToBP_BloodM (.HitActor (Collision|BreakHitResult _outhit))))
      (Default|LowerOpacity _asbp_blood_m))))

(event EventBeginPlay
  (Utilities|Time|SetTimerbyEvent (EventDispatchers|CreateEvent :!event Custom|Patata) 2.0 true))

(fn ConstructionScript)