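; BP_Fregona is a mop actor that cleans blood beneath it.
; BeginPlay starts a looping timer, apparently driving the Patata event, which line-traces a short distance straight down from the actor with persistent debug drawing.
; When the hit actor is tagged Blood and casts to BP_BloodM, it calls LowerOpacity on it to fade the stain.
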(event Custom|Patata
  (bind _returnvalue (Transformation|GetActorLocation))
  (bind (_outhit _returnvalue_2) (Collision|LineTraceByChannel _returnvalue (+ _returnvalue (* (Math|Vector|VectorUp) -3e+01)) "TraceTypeQuery1" true 0 "Persistent"))
  (if _returnvalue_2
    (if (Actor|ActorHasTag (.HitActor (Collision|BreakHitResult _outhit)) "Blood")
      (bind _asbp_blood_m (Utilities|Casting|CastToBP_BloodM (.HitActor (Collision|BreakHitResult _outhit))))
      (Default|LowerOpacity _asbp_blood_m))))

(event EventBeginPlay
  (Utilities|Time|SetTimerbyEvent (EventDispatchers|CreateEvent :!event Custom|Patata) 2.0 true))

(fn ConstructionScript)